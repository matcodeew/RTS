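; Selectable, movable unit that shows a selection decal while selected and travels to commanded locations.
; SelectUnit and DeselectUnit toggle the decal, which starts hidden.
; SetNewTargetLocation picks a random point in a small horizontal box around the given location, so the exact destination varies.
; While moving, Tick calls MoveTo at the Stat movement speed until the unit is within a distance threshold of the target.
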(event `self.ReceiveBeginPlay`
  (`SceneComponent.SetVisibility` (`self.SelectionDecal`) false false))

(event `/Game/Blueprint/Player/RTS_Interface.SelectUnit`
  (`SceneComponent.SetVisibility` (`self.SelectionDecal`) true false))

(event `/Game/Blueprint/Player/RTS_Interface.DeselectUnit`
  (`SceneComponent.SetVisibility` (`self.SelectionDecal`) false false))

(event `/Game/Blueprint/Player/RTS_Interface.SetNewTargetLocation`
  (params (Location :type "Vector Structure"))
  (set `self.DistanceTreshHold` 5.0)
  (set `self.TargetLocation` (`KismetMathLibrary.RandomPointInBoundingBox` Location (50.0 50.0 0.0)))
  (set `self.isMoving` true))

(event `self.ReceiveTick`
  (params (DeltaSeconds :type "Float (single-precision)"))
  (bind (_stat_name _stat_attackdamage _stat_maxlife _stat_currentlife _stat_movementspeed) (break `Struct_UnitStat` (`self.Stat`)))
  (if (`self.isMoving`)
    (`self.MoveTo` (`self.TargetLocation`) DeltaSeconds _stat_movementspeed)
    (if (< (`KismetMathLibrary.Vector_Distance` (`self.K2_GetActorLocation`) (`self.TargetLocation`)) (`self.DistanceTreshHold`))
      (set `self.isMoving` false))))

(fn `UserConstructionScript`)