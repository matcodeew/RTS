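; Base unit Blueprint that can be selected and ordered to move to a location.
; A selection decal starts hidden at BeginPlay and is shown or hidden by the select and deselect events.
; The move command stops the AI controller's current movement, then issues AIMoveTo to the new location, printing debug messages for the outcome or a missing controller.
; GrabSelectedUnit is an empty stub.
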(event `self.ReceiveBeginPlay`
  (`SceneComponent.SetVisibility` (`self.SelectionDecal`) false false))

(event `/Game/Blueprint/Controller/I_Marquee.SelectUnit`
  (`SceneComponent.SetVisibility` (`self.SelectionDecal`) true false))

(event `/Game/Blueprint/Controller/I_Marquee.DeselectUnit`
  (`SceneComponent.SetVisibility` (`self.SelectionDecal`) false false))

(event `/Game/Blueprint/Controller/I_Marquee.UnitMoveCommand`
  (params (location :type "Vector Structure"))
  (bind _returnvalue (`AIBlueprintHelperLibrary.GetAIController` self))
  (`/Engine/EditorBlueprintResources/StandardMacros.IsValid` _returnvalue
    (:`Is Valid`
      (`Controller.StopMovement` _returnvalue)
      (`AITask_MoveTo.AIMoveTo` _returnvalue location null 3.0
        (:`then`
          (`KismetSystemLibrary.PrintString` "Movement started"))
        (:`OnRequestFailed`
          (`KismetSystemLibrary.PrintString` "Request Failed"))
        (:`OnMoveFinished`
          (`KismetSystemLibrary.PrintString` "Move Finished"))))
    (:`Is Not Valid`
      (`KismetSystemLibrary.PrintString` "IA Controller is not valid" true true (struct :`R` 1.0 :`B` 0.060021 :`A` 1.0)))))

(fn `GrabSelectedUnit`
  (returns (Units :type "Array of Actor Object Reference"))
  (return))

(fn `UserConstructionScript`)