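; Enemy spawner that fills the level with a random mix of enemy units shortly after play begins.
; BeginPlay initializes the enemy pool, waits briefly, then loops over the pool size, printing each index as it goes.
; Each iteration randomly picks one of four enemy types and spawns it at a random X/Y position within a square range.
; The random roll has a fifth outcome with no case, so some iterations spawn nothing.
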(event `self.ReceiveBeginPlay`
  (bind _pool_size (`self.Pool Size`))
  (`AC_EnemyPool.InitializePool` (`self.EnemyPool`) _pool_size)
  (`KismetSystemLibrary.Delay` 2.5)
  (for _index (range (+ _pool_size 1))
    (`KismetSystemLibrary.PrintString` (`KismetStringLibrary.Conv_IntToString` _index))
    (switch `int` (`KismetMathLibrary.RandomIntegerInRange` 0 4)
      (:`0`
        (set `self.Type` "B_FanaticDevotee"))
      (:`1`
        (set `self.Type` "B_AbyssDogs"))
      (:`2`
        (set `self.Type` "B_ChainedBeasts"))
      (:`3`
        (set `self.Type` "B_ShootersFromTheAbyss")))
    (`self.SpawnEnemy` (`self.Type`) (`KismetMathLibrary.MakeVector` (`KismetMathLibrary.RandomFloatInRange` -200.0 200.0) (`KismetMathLibrary.RandomFloatInRange` -200.0 200.0)))))

(fn `UserConstructionScript`)