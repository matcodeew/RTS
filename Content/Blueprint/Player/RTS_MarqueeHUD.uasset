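; RTS HUD that handles marquee drag-selection of Unit actors and relays move orders to the selected units.
; Marquee press, hold and release events track the mouse corners and the drawing state.
; While dragging, DrawHUD draws a translucent rectangle and each frame selects fully enclosed units and deselects those outside via messages.
; SetNewTargetLocation forwards a destination to every non-hidden unit in the selection list.
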(event `/Game/Blueprint/Player/RTS_Interface.MarqueePressed`
  (bind (_locationx _locationy) (`PlayerController.GetMousePosition` (`GameplayStatics.GetPlayerController` 0)))
  (set `self.isDrawing` true)
  (bind _output_get (set `self.StartMousePosition` (`KismetMathLibrary.MakeVector2D` _locationx _locationy)))
  (set `self.CurrentMousePosition` _output_get))

(event `/Game/Blueprint/Player/RTS_Interface.MarqueeHold`
  (bind (_locationx _locationy) (`PlayerController.GetMousePosition` (`GameplayStatics.GetPlayerController` 0)))
  (set `self.CurrentMousePosition` (`KismetMathLibrary.MakeVector2D` _locationx _locationy)))

(event `/Game/Blueprint/Player/RTS_Interface.SetNewTargetLocation`
  (params (Location :type "Vector Structure"))
  (if (> (`KismetArrayLibrary.Array_Length` (`self.SelectedUnits`)) 0)
    (for _array_element (`self.SelectedUnits`)
      (if (not (`Actor.bHidden` _array_element))
        (message `/Game/Blueprint/Player/RTS_Interface.SetNewTargetLocation` _array_element Location)))))

(event `/Game/Blueprint/Player/RTS_Interface.MarqueeReleased`
  (set `self.isDrawing` false))

(event `self.ReceiveDrawHUD`
  (params (SizeX :type Integer) (SizeY :type Integer))
  (bind (_startmouseposition_x _startmouseposition_y) (`KismetMathLibrary.BreakVector2D` (`self.StartMousePosition`)))
  (bind (_currentmouseposition_x _currentmouseposition_y) (`KismetMathLibrary.BreakVector2D` (`self.CurrentMousePosition`)))
  (if (`self.isDrawing`)
    (`self.DrawRect` (struct :`R` 1.0 :`G` 0.05086 :`B` 0.967012 :`A` 0.323) _startmouseposition_x _startmouseposition_y (- _currentmouseposition_x _startmouseposition_x) (- _currentmouseposition_y _startmouseposition_y))
    (bind _output_get (set `self.UnitInRectangle` (`self.GetActorsInSelectionRectangle` "/Game/Blueprint/Units/Unit.Unit_C" (`self.StartMousePosition`) (`self.CurrentMousePosition`) true true)))
    (for _array_element _output_get
      (message `/Game/Blueprint/Player/RTS_Interface.SelectUnit` _array_element)
      (`KismetArrayLibrary.Array_AddUnique` (`self.SelectedUnits`) _array_element))
    (for _array_element_2 (`self.SelectedUnits`)
      (if (== (`KismetArrayLibrary.Array_Find` (`self.UnitInRectangle`) _array_element_2) -1)
        (message `/Game/Blueprint/Player/RTS_Interface.DeselectUnit` _array_element_2)
        (`KismetArrayLibrary.Array_RemoveItem` (`self.SelectedUnits`) _array_element_2)))))

(fn `UserConstructionScript`)