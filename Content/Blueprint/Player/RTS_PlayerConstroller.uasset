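; RTS player controller that turns mouse input into marquee selection and target-location commands, with a visible cursor in Game and UI input mode.
; Left-button press, hold (polled on Tick) and release are forwarded to the HUD as marquee messages.
; Right-click runs a short Visibility trace from the deprojected cursor, prints the location and sends it to the HUD as the new target, without checking for a hit.
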(event `self.ReceiveBeginPlay`
  (`WidgetBlueprintLibrary.SetInputMode_GameAndUIEx` self null "DoNotLock" false)
  (set `self.bShowMouseCursor` true))

(event `Key|LeftMouseButton`
  (params (Key :type "Key Structure"))
  (bind _returnvalue (`self.GetHUD`))
  (:`Pressed`
    (set `self.LeftMousePressed` true)
    (message `/Game/Blueprint/Player/RTS_Interface.MarqueePressed` _returnvalue))
  (:`Released`
    (set `self.LeftMousePressed` false)
    (message `/Game/Blueprint/Player/RTS_Interface.MarqueeReleased` _returnvalue)))

(event `Key|RightMouseButton`
  (params (Key :type "Key Structure"))
  (bind (_worldlocation _worlddirection) (`self.DeprojectMousePositionToWorld` (`GameplayStatics.GetPlayerController` 0)))
  (:`Pressed`
    (bind _outhit (`KismetSystemLibrary.LineTraceSingle` _worldlocation (+ _worldlocation (* (`KismetMathLibrary.GetForwardVector` (`KismetMathLibrary.Conv_VectorToRotator` _worlddirection)) 1500.0)) "TraceTypeQuery1"))
    (bind (_bblockinghit _binitialoverlap _time _distance _location) (`GameplayStatics.BreakHitResult` _outhit))
    (`KismetSystemLibrary.PrintString` (`KismetStringLibrary.Conv_VectorToString` _location))
    (message `/Game/Blueprint/Player/RTS_Interface.SetNewTargetLocation` (`self.GetHUD`) _location)))

(event `self.ReceiveTick`
  (params (DeltaSeconds :type "Float (single-precision)"))
  (if (`self.LeftMousePressed`)
    (message `/Game/Blueprint/Player/RTS_Interface.MarqueeHold` (`self.GetHUD`))))

(fn `UserConstructionScript`)