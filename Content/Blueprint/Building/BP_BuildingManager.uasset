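; BP_BuildingManager places buildings in the game from a requested building type and location.
; Its BuildBuilding event calls Build, stores the location on the resulting BP_Building, and sets that building's Core mesh and scale from its BuildingStat.
; It then resets TypeBuilding on the player's PC_Controller to None.
; GrabSelectedUnit is an empty stub, and the construction script does nothing.
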(event `/Game/Blueprint/Controller/I_Marquee.BuildBuilding`
  (params (`Building Type` :type "EEnum_BuildingType Enum" :default "None") (Location :type "Vector Structure"))
  ;[0.04171 0.03272 0.15 0.5] Create Building and Set Static mesh and mesh Scale
  (bind _returnvalue (`self.Build` `Building Type` Location))
  (bind _asbp_building (cast `/Game/Blueprint/Building/BP_Building` _returnvalue))
  (`/Game/Blueprint/Building/BP_Building.SetVarLocation` _asbp_building Location)
  (bind _core (`/Game/Blueprint/Building/BP_Building.Core` _asbp_building))
  (bind (_buildingstat_buildingname _buildingstat_faithvalue _buildingstat_staticmesh _buildingstat_scalingvalue) (break `Struct_BuildingStat` (`ABuilding.BuildingStat` _asbp_building)))
  (`StaticMeshComponent.SetStaticMesh` _core _buildingstat_staticmesh)
  (`SceneComponent.SetWorldScale3D` _core _buildingstat_scalingvalue)
  ;[0.15 0.02494 0.0342 0.5] Set Building type to none
  (bind _aspc_controller (cast `/Game/Blueprint/Controller/PC_Controller` (`GameplayStatics.GetPlayerController` 0)))
  (set `/Game/Blueprint/Controller/PC_Controller.TypeBuilding` "None" _aspc_controller))

(fn `GrabSelectedUnit`
  (returns (Units :type "Array of Actor Object Reference"))
  (return))

(fn `UserConstructionScript`)