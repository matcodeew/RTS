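; Spawner building that produces units from a pooled enemy component and offers a unit-creation menu when interacted with.
; BeginPlay initializes the pool, and OnSpawnUnit takes a unit of the requested type, moves it to a random point around the building, then applies gravity plus the mesh and walk speed from its stats.
; Interaction opens the menu widget with unit icons gathered from the pool's type-to-data map and a resource icon array.
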(event `self.ReceiveBeginPlay`
  (`AC_EnemyPool.InitializePool` (`self.AC_EnemyPool`) (`self.PoolSize`) (0.0 0.0 300.0)))

(event `/Game/Blueprint/Controller/I_Marquee.OnSpawnUnit`
  (params (`Unit Type` :type "EEnum_UnitType Enum" :default "None"))
  (bind (_returnvalue_x _returnvalue_y) (`KismetMathLibrary.BreakVector` (`KismetMathLibrary.RandomPointInBoundingBox` (`self.K2_GetActorLocation` self) (150.0 150.0 0.0))))
  (bind _enemy (`self.SpawnEnemy` `Unit Type` (`KismetMathLibrary.MakeVector` _returnvalue_x _returnvalue_y)))
  (`/Engine/EditorBlueprintResources/StandardMacros.IsValid` _enemy
    (:`Is Valid`
      (set `CharacterMovementComponent.GravityScale` 1.0 (`Character.CharacterMovement` _enemy))
      (bind (_stat_name _stat_attackdamage _stat_maxlife _stat_currentlife _stat_movementspeed _stat_spawnrate _stat_ressourcevalue _stat_skeletalmesh) (break `Struct_UnitStat` (`AUnit.Stat` _enemy)))
      (`SkeletalMeshComponent.SetSkeletalMeshAsset` (`Character.Mesh` _enemy) _stat_skeletalmesh)
      (set `CharacterMovementComponent.MaxWalkSpeed` _stat_movementspeed (`Character.CharacterMovement` _enemy)))))

(event `/Game/Blueprint/Controller/I_Marquee.InteractWithBuilding`
  (params (Units :type "/Game/Blueprint/Units/BP_UnitParent Object Reference"))
  (`KismetSystemLibrary.PrintString` "Interact with Spawner")
  (bind _returnvalue (`|CreateWidget` "/Game/WidgetUI/UnitsUI/WD_CreateUnitsMenu.WD_CreateUnitsMenu_C"))
  (bind (_new_unit_icon_array _new_ressource_icon_array) (`self.Set Array `))
  (`/Game/WidgetUI/UnitsUI/WD_CreateUnitsMenu.InitializeUnitCase` _returnvalue _new_unit_icon_array _new_ressource_icon_array)
  (`UserWidget.AddToPlayerScreen` _returnvalue 0))

(fn `Set Array `
  (returns (`new Unit Icon Array` :type "Array of Texture2D Object Reference") (`new Ressource Icon Array` :type "Array of Texture2D Object Reference"))
  (bind _values (`BlueprintMapLibrary.Map_Values` (`AC_EnemyPool.UnitTypeToDataMap` (`self.AC_EnemyPool`))))
  (for _array_element _values
    (`KismetArrayLibrary.Array_AddUnique` (`self.Unit Icon`) (`DA_Unit.UnitIcon` _array_element)))
  (return (`self.Unit Icon`) (`self.Ressource Icon`)))

(fn `Set Enemy Type With Index`
  (params (`Type Index` :type Integer))
  (returns (EnemyType :type "EEnum_UnitType Enum"))
  (switch `int` `Type Index`
    (:`0`
      (set `self.Type` "B_FanaticDevotee"))
    (:`1`
      (set `self.Type` "B_AbyssDogs"))
    (:`2`
      (set `self.Type` "B_ChainedBeasts"))
    (:`3`
      (set `self.Type` "B_AbyssShooter")))
  (return (`self.Type`)))

(fn `SpawnEnemy`
  (params (`Unity type` :type "EEnum_UnitType Enum" :default "None") (Position :type "Vector Structure"))
  (returns (Enemy :type "AUnit Object Reference"))
  (`/Engine/EditorBlueprintResources/StandardMacros.IsValid` (`self.AC_EnemyPool`)
    (:`Is Valid`
      (bind _returnvalue (`AC_EnemyPool.GetEnemyFromPool` (`self.AC_EnemyPool`) `Unity type`))
      (`/Engine/EditorBlueprintResources/StandardMacros.IsValid` _returnvalue
        (:`Is Valid`
          (`self.K2_SetActorLocation` _returnvalue Position false false)
          (return _returnvalue))
        (:`Is Not Valid`
          (return null))))
    (:`Is Not Valid`
      (return null))))

(fn `UserConstructionScript`
  (`parent.UserConstructionScript`))