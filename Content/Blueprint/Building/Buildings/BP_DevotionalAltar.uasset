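; BP_DevotionalAltar is a building where units take prayer spots and generate Faith over time.
; Interact gathers spot locations from PrayerPosParent's children, teleports the unit to the last free one and records it in the PositionOccupied map.
; A Tick timer periodically adds Faith to BP_RessourceManager in proportion to the number of occupants.
; ResetPrayerPlaces frees a unit's spot by removing its map entry.
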(event `self.ReceiveTick`
  (params (DeltaSeconds :type "Float (single-precision)"))
  (bind _timer (`self.timer`))
  ;[0.1337 0.03481 0.15 0.5] Timer
  (set `self.timer` (+ DeltaSeconds _timer))
  (if (>= _timer (`self.TimeToWait`))
    (set `self.timer` 0.0)
    (bind _keys (`BlueprintMapLibrary.Map_Keys` (`self.PositionOccupied`)))
    (bind _returnvalue (`GameplayStatics.GetActorOfClass` "/Game/Blueprint/Controller/BP_RessourceManager.BP_RessourceManager_C"))
    (`/Game/Blueprint/Controller/BP_RessourceManager.AddingFaith` _returnvalue (* 0.25 (`KismetArrayLibrary.Array_Length` _keys)))))

(fn `GetPrayerPos`
  (params (location :type "Vector Structure"))
  (for _array_element (`SceneComponent.GetChildrenComponents` (`self.PrayerPosParent`) false)
    (`KismetArrayLibrary.Array_AddUnique` (`self.PrayerPositions `) (`SceneComponent.K2_GetComponentLocation` _array_element))))

(fn `Interact`
  (params (Unit :type "Actor Object Reference"))
  (returns (OutPutUnit :type "Array of Actor Object Reference"))
  (bind _unitoutput (`self.UnitOutput`))
  (bind _position (`self.position`))
  (`self.GetPrayerPos` (`self.BuildingWorldPos`))
  (bind _values (`BlueprintMapLibrary.Map_Values` (`self.PositionOccupied`)))
  (if (< (`KismetArrayLibrary.Array_Length` _values) (`KismetArrayLibrary.Array_Length` (`self.PrayerPositions `)))
    (for _array_element (`self.PrayerPositions `)
      (bind _values_2 (`BlueprintMapLibrary.Map_Values` (`self.PositionOccupied`)))
      (if (not (`KismetArrayLibrary.Array_Contains` _values_2 _array_element))
        (set `self.position` _array_element)))
    (`self.K2_SetActorLocation` Unit _position false false)
    (`BlueprintMapLibrary.Map_Add` (`self.PositionOccupied`) Unit _position)
    (`KismetArrayLibrary.Array_AddUnique` _unitoutput Unit)
    (return _unitoutput)))

(fn `ResetPrayerPlaces`
  (params (UnitToRemove :type "Actor Object Reference"))
  (if (`BlueprintMapLibrary.Map_Contains` (`self.PositionOccupied`) UnitToRemove)
    (`BlueprintMapLibrary.Map_Remove` (`self.PositionOccupied`) UnitToRemove)))

(fn `UserConstructionScript`
  (`parent.UserConstructionScript`))