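; BP_Spawner is a building that fills the area around itself with random enemies and opens a unit-creation menu when interacted with.
; On BeginPlay it initializes an enemy pool, waits briefly, then loops over the pool size, picking among four enemy types; a fifth random result spawns nothing.
; Each valid spawn gets its skeletal mesh and walk speed from its stats.
; Interaction adds WD_CreateUnitsMenu to the player screen, while GrabSelectedUnit is empty.
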(event `self.ReceiveBeginPlay`
  (bind _poolsize (`self.PoolSize`))
  (bind (_returnvalue_x _returnvalue_y) (`KismetMathLibrary.BreakVector` (`KismetMathLibrary.RandomPointInBoundingBox` (`self.K2_GetActorLocation` self) (150.0 150.0 0.0))))
  (`AC_EnemyPool.InitializePool` (`self.EnemyPool`) _poolsize)
  (`KismetSystemLibrary.Delay` 1.5)
  (for _ (range (+ _poolsize 1))
    (switch `int` (`KismetMathLibrary.RandomIntegerInRange` 0 4)
      (:`0`
        (set `self.Type` "B_FanaticDevotee"))
      (:`1`
        (set `self.Type` "B_AbyssDogs"))
      (:`2`
        (set `self.Type` "B_ChainedBeasts"))
      (:`3`
        (set `self.Type` "B_ShootersFromTheAbyss")))
    (bind _returnvalue (`self.SpawnEnemy` (`self.Type`) (`KismetMathLibrary.MakeVector` _returnvalue_x _returnvalue_y 30.0)))
    (`/Engine/EditorBlueprintResources/StandardMacros.IsValid` _returnvalue
      (:`Is Valid`
        (bind (_stat_name _stat_attackdamage _stat_maxlife _stat_currentlife _stat_movementspeed _stat_spawnrate _stat_ressourcevalue _stat_skeletalmesh) (break `Struct_UnitStat` (`AUnit.Stat` _returnvalue)))
        (`SkeletalMeshComponent.SetSkeletalMeshAsset` (`Character.Mesh` _returnvalue) _stat_skeletalmesh)
        (set `CharacterMovementComponent.MaxWalkSpeed` _stat_movementspeed (`Character.CharacterMovement` _returnvalue))))))

(event `/Game/Blueprint/Controller/I_Marquee.InteractWithBuilding`
  (params (Units :type "/Game/Blueprint/Units/BP_UnitParent Object Reference"))
  (bind _returnvalue (`|CreateWidget` "/Game/WidgetUI/UnitsUI/WD_CreateUnitsMenu.WD_CreateUnitsMenu_C"))
  (`UserWidget.AddToPlayerScreen` _returnvalue 0))

(fn `GrabSelectedUnit`
  (returns (Units :type "Array of Actor Object Reference"))
  (return))

(fn `UserConstructionScript`)