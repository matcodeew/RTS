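; BP_Building is a building Blueprint that responds to units interacting with it, branching on its building type.
; The InteractwithBuilding event stores the passed units and routes a Devotional Altar to its own behaviour function, while a None type only prints a warning.
; The altar behaviour is a stub that loops over the units without acting and prints a debug message; GrabSelectedUnit is empty.
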(event `/Game/Blueprint/Controller/I_Marquee.InteractWithBuilding`
  (params (Units :type "Array of /Game/Blueprint/Units/BP_UnitParent Object Reference (by ref)"))
  (set `self.Units` Units)
  (`KismetSystemLibrary.PrintString` "Hello")
  (switch `EEnum_BuildingType` (`self.BuildingType`)
    (:`None`
      (`KismetSystemLibrary.PrintString` "The Building Type is null" true true (struct :`R` 1.0 :`G` 0.003962 :`A` 1.0) 10.0))
    (:`DevotionalAltar`
      (`self.DevotionalAltar Behaviour` (`self.Units`)))))

(fn `DevotionalAltar Behaviour`
  (params (Units :type "Array of /Game/Blueprint/Units/BP_UnitParent Object Reference"))
  (for _ Units
    _)
  (`KismetSystemLibrary.PrintString` "All Actor move arround building"))

(fn `GrabSelectedUnit`
  (returns (Units :type "Array of Actor Object Reference"))
  (return))

(fn `UserConstructionScript`)