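; BP_MarqueeHUD is a HUD that provides drag-box unit selection.
; Pressed, hold and released events track the start and current mouse positions and whether the box is drawn.
; While drawing, DrawHUD renders a translucent rectangle, messages actors inside to select, and deselects and removes those outside, editing ActorSelected while looping over it.
; GrabSelectedUnit returns that selection list.
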(event `/Game/Blueprint/Controller/I_Marquee.MarqueReleased`
  (set `self.IsDrawing` false))

(event `/Game/Blueprint/Controller/I_Marquee.MarqueePressed`
  (bind (_locationx _locationy) (`PlayerController.GetMousePosition` (`GameplayStatics.GetPlayerController` 0)))
  (set `self.IsDrawing` true)
  (bind _output_get (set `self.StartMousePosition` (`KismetMathLibrary.MakeVector2D` _locationx _locationy)))
  (set `self.CurrentMousePosition` _output_get))

(event `/Game/Blueprint/Controller/I_Marquee.MarqueeHold`
  (bind (_locationx _locationy) (`PlayerController.GetMousePosition` (`GameplayStatics.GetPlayerController` 0)))
  (set `self.CurrentMousePosition` (`KismetMathLibrary.MakeVector2D` _locationx _locationy)))

(event `self.ReceiveDrawHUD`
  (params (SizeX :type Integer) (SizeY :type Integer))
  (bind (_startmouseposition_x _startmouseposition_y) (`KismetMathLibrary.BreakVector2D` (`self.StartMousePosition`)))
  (bind (_currentmouseposition_x _currentmouseposition_y) (`KismetMathLibrary.BreakVector2D` (`self.CurrentMousePosition`)))
  (if (`self.IsDrawing`)
    (`self.DrawRect` (struct :`R` 0.283428 :`G` 0.132188 :`B` 0.318547 :`A` 0.376) _startmouseposition_x _startmouseposition_y (- _currentmouseposition_x _startmouseposition_x) (- _currentmouseposition_y _startmouseposition_y))
    (bind _output_get (set `self.ActorInSelectionRect` (`self.GetActorsInSelectionRectangle` "/Script/Engine.Actor" (`self.StartMousePosition`) (`self.CurrentMousePosition`) false)))
    (for _array_element _output_get
      (message `/Game/Blueprint/Controller/I_Marquee.SelectUnit` _array_element)
      (`KismetArrayLibrary.Array_AddUnique` (`self.ActorSelected`) _array_element))
    (for _array_element_2 (`self.ActorSelected`)
      (if (== (`KismetArrayLibrary.Array_Find` (`self.ActorInSelectionRect`) _array_element_2) -1)
        (message `/Game/Blueprint/Controller/I_Marquee.DeselectUnit` _array_element_2)
        (`KismetArrayLibrary.Array_RemoveItem` (`self.ActorSelected`) _array_element_2)))))

(fn `GrabSelectedUnit`
  (returns (Units :type "Array of Actor Object Reference"))
  (return (`self.ActorSelected`)))

(fn `UserConstructionScript`)