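; RTS player controller that sets up the cursor and building menu and edge-scrolls the camera pawn.
; Left mouse drives marquee selection through HUD messages.
; Right-click traces under the cursor and picks a command from pending building type, hit building and HUD-selected units: build via BP_BuildingManager, interact, or move units with a cursor effect.
; Interact only prints the actor name and moves units; the InteractWithBuilding call is unconnected.
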(event `self.ReceiveBeginPlay`
  ; Get BP_Camera
  (`WidgetBlueprintLibrary.SetInputMode_GameAndUIEx` self null "LockAlways" false)
  (set `self.bShowMouseCursor` true)
  (bind _asbp_camera (cast `/Game/Blueprint/Player/BP_Camera` (`self.K2_GetPawn`)))
  (set `self.CameraSpringArms` (`/Game/Blueprint/Player/BP_Camera.SpringArm` _asbp_camera))
  (bind _returnvalue (`|CreateWidget` "/Game/WidgetUI/WB_BuildingMenu.WB_BuildingMenu_C"))
  (`UserWidget.AddToPlayerScreen` _returnvalue 0))

(event `InputAxisKey|MouseX`
  (params (AxisValue :type "Float (single-precision)"))
  (bind _returnvalue_x (`KismetMathLibrary.BreakVector2D` (`WidgetLayoutLibrary.GetViewportSize`)))
  (bind _returnvalue (`self.K2_GetPawn`))
  (bind _returnvalue_2 (/ (`self.GetMousePosition`) _returnvalue_x))
  (bind _returnvalue_3 (* (`self.ScrollSpeed`) (`GameplayStatics.GetWorldDeltaSeconds`)))
  ; Move Camera when the mouse cross the screen size
  (if (> _returnvalue_2 0.98)
    (`self.K2_AddActorWorldOffset` _returnvalue (`KismetMathLibrary.MakeVector` 0.0 _returnvalue_3) false false)
    (elif (< _returnvalue_2 0.02)
      (`self.K2_AddActorWorldOffset` _returnvalue (`KismetMathLibrary.MakeVector` 0.0 (* _returnvalue_3 -1.0)) false false))))

(event `InputAxisKey|MouseY`
  (params (AxisValue :type "Float (single-precision)"))
  (bind _returnvalue (`self.K2_GetPawn`))
  (bind (_returnvalue_x _returnvalue_y) (`KismetMathLibrary.BreakVector2D` (`WidgetLayoutLibrary.GetViewportSize`)))
  (bind _returnvalue_2 (/ (`.LocationY` (`self.GetMousePosition`)) _returnvalue_y))
  (bind _returnvalue_3 (* (`self.ScrollSpeed`) (`GameplayStatics.GetWorldDeltaSeconds`)))
  ; Move Camera when the mouse cross the screen size
  (if (> _returnvalue_2 0.98)
    (`self.K2_AddActorWorldOffset` _returnvalue (`KismetMathLibrary.MakeVector` (* _returnvalue_3 -1.0)) false false)
    (elif (< _returnvalue_2 0.02)
      (`self.K2_AddActorWorldOffset` _returnvalue (`KismetMathLibrary.MakeVector` _returnvalue_3) false false))))

(event `self.ReceiveTick`
  (params (DeltaSeconds :type "Float (single-precision)"))
  (if (`self.LeftMouseButtonHold`)
    (message `/Game/Blueprint/Controller/I_Marquee.MarqueeHold` (`self.GetHUD`))))

(event `Key|LeftMouseButton`
  (params (Key :type "Key Structure"))
  (bind _returnvalue (`self.GetHUD`))
  (:`Pressed`
    (set `self.LeftMouseButtonHold` true)
    (message `/Game/Blueprint/Controller/I_Marquee.MarqueePressed` _returnvalue))
  (:`Released`
    (set `self.LeftMouseButtonHold` false)
    (message `/Game/Blueprint/Controller/I_Marquee.MarqueReleased` _returnvalue)))

(event `Key|RightMouseButton`
  (params (Key :type "Key Structure"))
  (bind (_bblockinghit _binitialoverlap _time _distance _location _impactpoint _normal _impactnormal _physmat _hitactor) (`GameplayStatics.BreakHitResult` (`self.GetHitResultUnderCursorByChannel` "TraceTypeQuery1")))
  (:`Pressed`
    (bind _clicked_state (`self.Update Click State` _hitactor))
    (set `self.ClickedEnum` _clicked_state)
    (set `self.RightClickLocation` _location)
    (switch `/Game/Blueprint/Controller/EClickedAction` (`self.ClickedEnum`)
      (:`NewEnumerator0`
        (`self.Move Units`))
      (:`NewEnumerator1`
        (`KismetSystemLibrary.PrintString` (`KismetSystemLibrary.GetDisplayName` _hitactor))
        (`self.Move Units`))
      (:`NewEnumerator2`
        (`self.Build Structure`)))
    (set `self.ClickedEnum` "NewEnumerator3")))

(fn `Build Structure`
  (bind _returnvalue (`GameplayStatics.GetActorOfClass` "/Game/Blueprint/Building/BP_BuildingManager.BP_BuildingManager_C"))
  (message `/Game/Blueprint/Controller/I_Marquee.BuildBuilding` _returnvalue (`self.TypeBuilding`) (`self.RightClickLocation`)))

(fn `GrabSelectedUnit`
  (returns (Units :type "Array of Actor Object Reference"))
  (return))

(fn `InteractWithBuilding`
  (params (Units :type "/Game/Blueprint/Units/BP_UnitParent Object Reference")))

(fn `Move Units`
  (bind _rightclicklocation (`self.RightClickLocation`))
  (bind _units (message `/Game/Blueprint/Controller/I_Marquee.GrabSelectedUnit` (`self.GetHUD`)))
  (for _array_element _units
    (message `/Game/Blueprint/Controller/I_Marquee.UnitMoveCommand` _array_element _rightclicklocation))
  (`NiagaraFunctionLibrary.SpawnSystemAtLocation` "/Game/Cursor/FX_Cursor.FX_Cursor" _rightclicklocation (struct) (0.75 0.75 0.75)))

(fn `Update Click State`
  (params (`Hited Actor` :type "Actor Object Reference"))
  (returns (`Clicked State` :type "/Game/Blueprint/Controller/EClickedAction Enum"))
  (bind _returnvalue (> (`KismetArrayLibrary.Array_Length` (`self.UnitsToMove`)) 0))
  (cast `/Game/Blueprint/Building/BP_Building` `Hited Actor`
    (:`then`
      (set `self.CastFailed` false))
    (:`CastFailed`
      (set `self.CastFailed` true)))
  (`KismetArrayLibrary.Array_Clear` (`self.UnitsToMove`))
  (bind _units (message `/Game/Blueprint/Controller/I_Marquee.GrabSelectedUnit` (`self.GetHUD`)))
  (for _array_element _units
    (bind _asbp_unit_parent (cast `/Game/Blueprint/Units/BP_UnitParent` _array_element))
    (`KismetArrayLibrary.Array_AddUnique` (`self.UnitsToMove`) _asbp_unit_parent))
  (if (`|EnumInequality` (`self.TypeBuilding`))
    (return "NewEnumerator2")
    (elif (and (not (`self.CastFailed`)) _returnvalue)
      (return "NewEnumerator1")
      (elif (and _returnvalue (`self.CastFailed`))
        (return "NewEnumerator0")
        (else
          (return "NewEnumerator3"))))))

(fn `UserConstructionScript`)